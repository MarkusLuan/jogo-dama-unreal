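; BP_TabGrid is one checkers board square that turns red when the mouse hovers over a valid selection.
; With no piece selected, painted squares highlight the current player's piece and tag it as hovered.
; With one selected, empty squares qualify as diagonal steps or jumps over an opponent, recording the captured piece on BP_Tabuleiro.
; Short line traces find neighbouring squares and pieces, while actor tags share hover and selection state.
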(event `self.ReceiveBeginPlay`
  (bind _returnvalue (`GameplayStatics.GetPlayerController` 0))
  (`self.EnableInput` _returnvalue)
  (set `PlayerController.bEnableMouseOverEvents` true _returnvalue))

(event `OnMouseOverPeca`
  (if (`self.IsPintado`) :!label _label
    (bind (_ispecaemcima _peca) (`self.IsPecaEmCima` self))
    (bind _outactors (`GameplayStatics.GetAllActorsOfClassWithTag` "/Game/Blueprints/BP_Peca.BP_Peca_C" "Selecionado"))
    (bind _returnvalue (`KismetArrayLibrary.Array_IsEmpty` _outactors))
    (if (xor (not _returnvalue) _ispecaemcima)
      (if _returnvalue
        (bind _returnvalue_2 (`GameplayStatics.GetActorOfClass` "/Game/Blueprints/Tabuleiro/BP_Tabuleiro.BP_Tabuleiro_C"))
        (bind _isplayerpreta (`/Game/Blueprints/Tabuleiro/BP_Tabuleiro.IsPlayerPreta` _returnvalue_2))
        (`self.SetSelecionado` (== _isplayerpreta (`/Game/Blueprints/BP_Peca.IsPreta` _peca)))
        (set `Actor.Tags` (`|MakeArray` "MouseEmCima" :!type "Name") _peca)
        (else
          (for _index (range 5)
            (bind _output (`|GetArrayItem` _outactors))
            (bind _returnvalue_3 (`self.K2_GetActorLocation` _output))
            (bind _returnvalue_4 (select `int` _index :`0` (80.0 80.0 0.0) :`1` (-80.0 80.0 0.0) :`2` (80.0 -80.0 0.0) :`3` (-80.0 -80.0 0.0) :!type "Vector Structure"))
            (bind (_isgriddiagonal _grid) (`self.IsGridDiagonal` (+ _returnvalue_3 _returnvalue_4 (0.0 0.0 -20.0))))
            (`|ExecutionSequence`
              (:`then_0`
                (if _isgriddiagonal
                  (`self.SetSelecionado` true :!label _label_2)
                  (bind _outactors_2 (`GameplayStatics.GetAllActorsOfClassWithTag` "BP_TabGrid_C" "Selecionado"))
                  (if (not (`KismetArrayLibrary.Array_IsEmpty` _outactors_2))
                    (`KismetArrayLibrary.Array_RemoveItem` (`Actor.Tags` (`|GetArrayItem` _outactors_2)) "Selecionado"))
                  (set `self.Tags` (`|MakeArray` "Selecionado" :!type "Name"))
                  (else
                    (bind _isgriddiagonal_2 (`self.IsGridDiagonal` (+ _returnvalue_3 (* _returnvalue_4 2) (0.0 0.0 -20.0))))
                    (`/Engine/EditorBlueprintResources/StandardMacros.IsValid` _grid
                      (:`Is Valid`
                        (bind (_ispecaemcima_2 _peca_2) (`self.IsPecaEmCima` _grid))
                        (`/Engine/EditorBlueprintResources/StandardMacros.IsValid` _peca_2
                          (:`Is Valid`
                            (if (and _ispecaemcima_2 _isgriddiagonal_2 (!= (`/Game/Blueprints/BP_Peca.IsPreta` _peca_2) (`/Game/Blueprints/BP_Peca.IsPreta` _output)))
                              (bind _returnvalue_5 (`GameplayStatics.GetActorOfClass` "/Game/Blueprints/Tabuleiro/BP_Tabuleiro.BP_Tabuleiro_C"))
                              (set `/Game/Blueprints/Tabuleiro/BP_Tabuleiro.PecaComida` _peca_2 _returnvalue_5)
                              (goto _label_2)))))))))
              (:`then_1`
                (if _isgriddiagonal
                  (break))))))))))

(event `self.ReceiveActorBeginCursorOver`
  (goto _label))

(event `OnMouseOutPeca`
  (bind _returnvalue (`self.K2_GetActorLocation` self))
  (`KismetArrayLibrary.Array_RemoveItem` (`self.Tags`) "Selecionado" :!label _label_3)
  (bind _outactors (`GameplayStatics.GetAllActorsOfClassWithTag` "/Game/Blueprints/BP_Peca.BP_Peca_C" "Selecionado"))
  (if (`KismetArrayLibrary.Array_IsEmpty` _outactors)
    (`self.SetSelecionado` false)
    (bind _outactors_2 (`GameplayStatics.GetAllActorsOfClassWithTag` "/Game/Blueprints/BP_Peca.BP_Peca_C" "MouseEmCima"))
    (if (`KismetArrayLibrary.Array_IsNotEmpty` _outactors_2)
      (`KismetArrayLibrary.Array_RemoveItem` (`Actor.Tags` (`|GetArrayItem` _outactors_2)) "MouseEmCima"))
    (else
      (bind _outhit (`KismetSystemLibrary.LineTraceSingle` :`Start` _returnvalue :`End` (+ _returnvalue (0.0 0.0 20.0)) :`TraceChannel` "TraceTypeQuery1" :`DrawDebugType` "ForDuration" :`DrawTime` 10.0))
      (if (not (== (`.HitActor` (`GameplayStatics.BreakHitResult` _outhit)) (`|GetArrayItem` _outactors)))
        (`self.SetSelecionado` false)))))

(event `self.ReceiveActorEndCursorOver`
  (goto _label_3))

(fn `IsGridDiagonal`
  (params (PosicaoCheck :type "Vector Structure"))
  (returns (IsGridDiagonal :type Boolean) (Grid :type "/Game/Blueprints/Tabuleiro/BP_TabGrid Object Reference"))
  (bind _outhit (`KismetSystemLibrary.LineTraceSingle` :`Start` PosicaoCheck :`End` (+ PosicaoCheck (1.0 1.0 0.0)) :`TraceChannel` "TraceTypeQuery1" :`DrawDebugType` "ForDuration" :`bIgnoreSelf` false :`DrawTime` 10.0))
  (bind _asbp_tab_grid (cast `/Game/Blueprints/Tabuleiro/BP_TabGrid` (`.HitActor` (`GameplayStatics.BreakHitResult` _outhit))))
  (return (== self (`.HitActor` (`GameplayStatics.BreakHitResult` _outhit))) _asbp_tab_grid))

(fn `IsPecaEmCima`
  (returns (IsPecaEmCima :type Boolean) (Peca :type "/Game/Blueprints/BP_Peca Object Reference"))
  (bind _returnvalue (`self.K2_GetActorLocation` self))
  (bind (_outhit _returnvalue_2) (`KismetSystemLibrary.LineTraceSingle` :`Start` _returnvalue :`End` (+ _returnvalue (0.0 0.0 20.0)) :`TraceChannel` "TraceTypeQuery1" :`DrawTime` 10.0))
  (bind _asbp_peca (cast `/Game/Blueprints/BP_Peca` (`.HitActor` (`GameplayStatics.BreakHitResult` _outhit)))
    (:`then`
      (return _returnvalue_2 _asbp_peca))
    (:`CastFailed`
      (return false null))))

(fn `SetSelecionado`
  (params (IsSelecionado :type Boolean))
  (`MeshComponent.SetVectorParameterValueOnMaterials` (`self.StaticMesh`) "Cor" (`KismetMathLibrary.Conv_LinearColorToVector` (`KismetMathLibrary.SelectColor` (struct :`R` 1.0 :`A` 1.0) (`KismetMathLibrary.SelectColor` (struct :`G` 0.078431 :`B` 0.286275 :`A` 1.0) (struct :`R` 1.0 :`G` 1.0 :`B` 1.0 :`A` 1.0) (`self.IsPintado`)) IsSelecionado))))

(fn `UserConstructionScript`
  (`self.SetSelecionado` false))