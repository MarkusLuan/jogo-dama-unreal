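; BP_Tabuleiro is the board actor for a two-player checkers game, spawning BP_TabGrid tiles and BP_Peca pieces in alternating patterns around its location.
; On left-click release it uses actor tags to select the active player's hovered piece or move the selected piece onto the selected tile.
; Moves destroy any captured piece and score it, check for a winning score to show the game-over UI, then switch player and flip the camera.
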(event `self.ReceiveBeginPlay`
  (`self.SpawnEixoX`)
  (`self.SpawnEixoY` (`self.K2_GetActorLocation` self) true)
  (set `PlayerController.bShowMouseCursor` true (`GameplayStatics.GetPlayerController` 0))
  (bind _returnvalue (`|CreateWidget` "/Game/UI/UI_Main.UI_Main_C" (`GameplayStatics.GetPlayerController` 0)))
  (`UserWidget.AddToViewport` _returnvalue 0))

(event `Key|LeftMouseButton`
  (params (Key :type "Key Structure"))
  (bind _pecacomida (`self.PecaComida`))
  (:`Released`
    (bind _outactors (`GameplayStatics.GetAllActorsOfClassWithTag` "/Game/Blueprints/BP_Peca.BP_Peca_C" "MouseEmCima"))
    (if (`KismetArrayLibrary.Array_IsEmpty` _outactors)
      (bind _outactors_2 (`GameplayStatics.GetAllActorsOfClassWithTag` "/Game/Blueprints/BP_Peca.BP_Peca_C" "Selecionado"))
      (if (not (`KismetArrayLibrary.Array_IsEmpty` _outactors_2))
        (bind _output (`|GetArrayItem` _outactors_2))
        (bind _grid (`/Game/Blueprints/BP_Peca.Grid` _output))
        (`/Engine/EditorBlueprintResources/StandardMacros.IsValid` _grid
          (:`Is Valid`
            (`/Game/Blueprints/Tabuleiro/BP_TabGrid.SetSelecionado` _grid false)
            (`KismetArrayLibrary.Array_RemoveItem` (`Actor.Tags` _output) "Selecionado")
            (bind _outactors_3 (`GameplayStatics.GetAllActorsOfClassWithTag` "/Game/Blueprints/Tabuleiro/BP_TabGrid.BP_TabGrid_C" "Selecionado"))
            (if (not (`KismetArrayLibrary.Array_IsEmpty` _outactors_3))
              (`self.K2_SetActorLocation` _output (+ (`self.K2_GetActorLocation` (`|GetArrayItem` _outactors_3)) (0.0 0.0 20.0)) false true)
              (`/Engine/EditorBlueprintResources/StandardMacros.IsValid` _pecacomida
                (:`Is Valid`
                  (`self.K2_DestroyActor` _pecacomida)
                  (`self.Comer Peca`))
                (:`Is Not Valid`
                  _))
              (`self.ChecarTemGanhador`)
              (`self.TrocarPlayer`)))))
      (else
        (bind _isplayerpreta (`self.IsPlayerPreta`))
        (bind _output_2 (`|GetArrayItem` _outactors))
        (if (== _isplayerpreta (`/Game/Blueprints/BP_Peca.IsPreta` _output_2))
          (bind _tags (`Actor.Tags` _output_2))
          (`KismetArrayLibrary.Array_Add` _tags "Selecionado")
          (`KismetArrayLibrary.Array_RemoveItem` _tags "MouseEmCima"))))))

(event `OnGanhar`
  (bind _returnvalue (`|CreateWidget` "/Game/UI/UI_Gameover.UI_Gameover_C"))
  (`UserWidget.AddToViewport` _returnvalue 0))

(fn `ChecarTemGanhador`
  (if (or (== (`self.ScorePreta`) 12) (== (`self.ScoreBranca`) 12))
    (`self.OnGanhar`)))

(fn `Comer Peca`
  (bind _isplayerpreta (`self.IsPlayerPreta`))
  (if _isplayerpreta
    (`/Engine/EditorBlueprintResources/StandardMacros.IncrementInt` (`self.ScorePreta`))
    (else
      (`/Engine/EditorBlueprintResources/StandardMacros.IncrementInt` (`self.ScoreBranca`)))))

(fn `IsPlayerPreta`
  (returns (IsPlayerPreta :type Boolean))
  (return (== (`self.PlayerAtivo`) 1)))

(fn `SpawnEixoX`
  (for _index (range 2)
    (for _index_2 (range 1 4)
      (bind _returnvalue (+ (* (`KismetMathLibrary.Conv_IntToVector` (* _index_2 (`KismetMathLibrary.SelectInt` 1 -1 (> _index 0)))) (100.0 0.0 0.0)) (`self.K2_GetActorLocation` self)))
      (bind _returnvalue_2 (== (mod _index_2 2) 0))
      (`self.SpawnEixoY` _returnvalue _returnvalue_2 :!label _label)
      (`self.SpawnGrid` _returnvalue _returnvalue_2)))
  (goto _label))

(fn `SpawnEixoY`
  (params (EixoX :type "Vector Structure") (`IsNãoPintado` :type Boolean))
  (locals (IsColocarCor :type Boolean) (DeveraGeraPeca :type Boolean) (Location :type "Vector Structure"))
  (bind _returnvalue (not (`local.IsColocarCor`)))
  (for _index (range 2)
    (set `local.IsColocarCor` (not `IsNãoPintado`))
    (for _index_2 (range 1 4)
      (bind _returnvalue_2 (> _index 0))
      (set `local.DeveraGeraPeca` (or (and (> _index_2 1) _returnvalue) (and _returnvalue (not _returnvalue_2))) :!label _label)
      (bind _output_get (set `local.Location` (+ EixoX (* (0.0 100.0 0.0) (`KismetMathLibrary.Conv_IntToVector` (* _index_2 (`KismetMathLibrary.SelectInt` 1 -1 _returnvalue_2)))))))
      (`self.SpawnGrid` _output_get (`local.IsColocarCor`))
      (set `local.IsColocarCor` (not (`local.IsColocarCor`)))
      (if (`local.DeveraGeraPeca`)
        (`self.SpawnPeca` (`local.Location`) (not (and (`local.IsColocarCor`) _returnvalue_2))))))
  (goto _label))

(fn `SpawnGrid`
  (params (Loc :type "Vector Structure") (IsNotGridPintado :type Boolean))
  (`|SpawnActorFromClass` "/Game/Blueprints/Tabuleiro/BP_TabGrid.BP_TabGrid_C" (`KismetMathLibrary.MakeTransform` Loc) "Undefined" "MultiplyWithRoot" self (not IsNotGridPintado) null))

(fn `SpawnPeca`
  (params (Loc :type "Vector Structure") (IsPecaPreta :type Boolean))
  (`|SpawnActorFromClass` "/Game/Blueprints/BP_Peca.BP_Peca_C" (`KismetMathLibrary.MakeTransform` (+ Loc (0.0 0.0 25.0))) "Undefined" "MultiplyWithRoot" null IsPecaPreta null))

(fn `TrocarPlayer`
  (bind _camera (`self.Camera`))
  (if (== (`self.PlayerAtivo`) 1)
    (set `self.PlayerAtivo` 2)
    (`SceneComponent.K2_SetRelativeRotation` _camera (struct :`Pitch` -90.0 :`Yaw` 270.0) false false)
    (else
      (set `self.PlayerAtivo` 1)
      (`SceneComponent.K2_SetRelativeRotation` _camera (struct :`Pitch` -90.0 :`Yaw` 90.0) false false))))

(fn `UserConstructionScript`)