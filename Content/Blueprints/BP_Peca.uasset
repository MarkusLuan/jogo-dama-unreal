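; BP_Peca is a board game piece that is either black or white and reports mouse hover to the grid square beneath it.
; On cursor over, a short downward line trace with debug drawing finds and stores the BP_TabGrid, which receives the mouse over and out calls.
; The construction script sets the cylinder's "Cor" material parameter from IsPreta, and SetCor overrides it.
; Older tag-based hover selection logic remains disconnected.
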(event `self.ReceiveActorBeginCursorOver`
  (bind _returnvalue (`self.K2_GetActorLocation` self))
  (bind _outhit (`KismetSystemLibrary.LineTraceSingle` :`Start` _returnvalue :`End` (- _returnvalue (0.0 0.0 20.0)) :`TraceChannel` "TraceTypeQuery1" :`DrawDebugType` "ForDuration" :`DrawTime` 10.0))
  (bind _asbp_tab_grid (cast `/Game/Blueprints/Tabuleiro/BP_TabGrid` (`.HitActor` (`GameplayStatics.BreakHitResult` _outhit))))
  (bind _output_get (set `self.Grid` _asbp_tab_grid))
  (`/Game/Blueprints/Tabuleiro/BP_TabGrid.OnMouseOverPeca` _output_get))

(event `self.ReceiveActorEndCursorOver`
  (bind _grid (`self.Grid`))
  (`/Engine/EditorBlueprintResources/StandardMacros.IsValid` _grid
    (:`Is Valid`
      (`/Game/Blueprints/Tabuleiro/BP_TabGrid.OnMouseOutPeca` _grid))))

(fn `SetCor`
  (params (Cor :type "LinearColor Structure"))
  (`MeshComponent.SetVectorParameterValueOnMaterials` (`self.Cylinder`) "Cor" (`KismetMathLibrary.Conv_LinearColorToVector` Cor)))

(fn `UserConstructionScript`
  (`MeshComponent.SetVectorParameterValueOnMaterials` (`self.Cylinder`) "Cor" (`KismetMathLibrary.Conv_LinearColorToVector` (`KismetMathLibrary.SelectColor` (struct) (struct :`R` 1.0 :`G` 1.0 :`B` 1.0 :`A` 1.0) (`self.IsPreta`)))))